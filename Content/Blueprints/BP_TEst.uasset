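; BP_TEst is a test pawn for AI navigation that walks toward a Goal location.
; On BeginPlay it casts its controller to AIController and issues a single MoveToLocation to the goal, with partial paths and stop-on-overlap disabled.
; Every Tick it prints the remaining distance to the goal as debug text.
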(event `self.ReceiveBeginPlay`
  (bind _asaicontroller (cast `AIController` (`self.GetController`)))
  (`AIController.MoveToLocation` _asaicontroller (.location (`self.goal`)) 0.0 false true false true null false))

(event `self.ReceiveTick`
  (params (DeltaSeconds :type "Float (single-precision)"))
  (`KismetSystemLibrary.PrintString` (`KismetStringLibrary.Concat_StrStr` "TEST : " (`KismetStringLibrary.Conv_DoubleToString` (`KismetMathLibrary.Vector_Distance` (.location (`self.goal`)) (`self.K2_GetActorLocation`))))))

(fn `UserConstructionScript`)