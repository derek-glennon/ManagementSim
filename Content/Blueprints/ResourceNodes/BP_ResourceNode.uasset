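; BP_ResourceNode is a resource node actor that offers up to four work locations to workers.
; BeginPlay gathers enabled WorkLocationComponents, and each one's overlap events set or clear its occupied flag.
; FindNearestAvailableWorkLocation searches them for the closest free spot to a worker position, returning its location and whether one was found.
; Cursor hover reveals child decals on free locations and hides them when the cursor leaves.
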(event `self.ReceiveBeginPlay`
  (add `self.OnBeginCursorOver` (`|CreateDelegate` :!event `OnBeginCursorOver_Event`))
  (add `self.OnEndCursorOver` (`|CreateDelegate` :!event `OnEndCursorOver_Event`))
  ;[1 0 0.003032] Create Work Locations Array
  (for _array_element (`self.K2_GetComponentsByClass` "/Script/ManagementSim.WorkLocationComponent")
    (if (`WorkLocationComponent.bIsEnabled` _array_element)
      (`KismetArrayLibrary.Array_Add` (`self.WorkLocations`) _array_element))))

(event `self.ReceiveTick`
  (params (DeltaSeconds :type "Float (single-precision)")))

(event `self.WorkLocation0.OnComponentBeginOverlap`
  (params (OverlappedComponent :type "PrimitiveComponent Object Reference") (OtherActor :type "Actor Object Reference") (OtherComp :type "PrimitiveComponent Object Reference") (OtherBodyIndex :type Integer) (bFromSweep :type Boolean) (SweepResult :type "HitResult Structure (by ref)"))
  ;[0 0.1048 1] Begin Overlap
  (`self.SetWorkLocationOccupied` OverlappedComponent true))

(event `self.WorkLocation1.OnComponentBeginOverlap`
  (params (OverlappedComponent :type "PrimitiveComponent Object Reference") (OtherActor :type "Actor Object Reference") (OtherComp :type "PrimitiveComponent Object Reference") (OtherBodyIndex :type Integer) (bFromSweep :type Boolean) (SweepResult :type "HitResult Structure (by ref)"))
  ;[0 0.1048 1] Begin Overlap
  (`self.SetWorkLocationOccupied` OverlappedComponent true))

(event `self.WorkLocation2.OnComponentBeginOverlap`
  (params (OverlappedComponent :type "PrimitiveComponent Object Reference") (OtherActor :type "Actor Object Reference") (OtherComp :type "PrimitiveComponent Object Reference") (OtherBodyIndex :type Integer) (bFromSweep :type Boolean) (SweepResult :type "HitResult Structure (by ref)"))
  ;[0 0.1048 1] Begin Overlap
  (`self.SetWorkLocationOccupied` OverlappedComponent true))

(event `self.WorkLocation3.OnComponentBeginOverlap`
  (params (OverlappedComponent :type "PrimitiveComponent Object Reference") (OtherActor :type "Actor Object Reference") (OtherComp :type "PrimitiveComponent Object Reference") (OtherBodyIndex :type Integer) (bFromSweep :type Boolean) (SweepResult :type "HitResult Structure (by ref)"))
  ;[0 0.1048 1] Begin Overlap
  (`self.SetWorkLocationOccupied` OverlappedComponent true))

(event `self.WorkLocation0.OnComponentEndOverlap`
  (params (OverlappedComponent :type "PrimitiveComponent Object Reference") (OtherActor :type "Actor Object Reference") (OtherComp :type "PrimitiveComponent Object Reference") (OtherBodyIndex :type Integer))
  ;[0 0.1048 1] End Overlap
  (`self.SetWorkLocationOccupied` OverlappedComponent))

(event `self.WorkLocation1.OnComponentEndOverlap`
  (params (OverlappedComponent :type "PrimitiveComponent Object Reference") (OtherActor :type "Actor Object Reference") (OtherComp :type "PrimitiveComponent Object Reference") (OtherBodyIndex :type Integer))
  ;[0 0.1048 1] End Overlap
  (`self.SetWorkLocationOccupied` OverlappedComponent))

(event `self.WorkLocation2.OnComponentEndOverlap`
  (params (OverlappedComponent :type "PrimitiveComponent Object Reference") (OtherActor :type "Actor Object Reference") (OtherComp :type "PrimitiveComponent Object Reference") (OtherBodyIndex :type Integer))
  ;[0 0.1048 1] End Overlap
  (`self.SetWorkLocationOccupied` OverlappedComponent))

(event `self.WorkLocation3.OnComponentEndOverlap`
  (params (OverlappedComponent :type "PrimitiveComponent Object Reference") (OtherActor :type "Actor Object Reference") (OtherComp :type "PrimitiveComponent Object Reference") (OtherBodyIndex :type Integer))
  ;[0 0.1048 1] End Overlap
  (`self.SetWorkLocationOccupied` OverlappedComponent))

(event `OnBeginCursorOver_Event` :!signature `self.OnBeginCursorOver`
  (params (TouchedActor :type "Actor Object Reference"))
  ;[0 0.1048 1] Set Visibility of Available Decal
  (for _array_element (`self.WorkLocations`)
    (if (`WorkLocationComponent.bIsEnabled` _array_element)
      (if (not (`WorkLocationComponent.bIsOccupied` _array_element))
        (for _array_element_2 (`SceneComponent.GetChildrenComponents` _array_element false)
          (bind _asdecal_component (cast `DecalComponent` _array_element_2))
          (`SceneComponent.SetVisibility` _asdecal_component true false))))))

(event `OnEndCursorOver_Event` :!signature `self.OnEndCursorOver`
  (params (TouchedActor :type "Actor Object Reference"))
  ;[0 0.1048 1] Set Visibility of Available Decal
  (for _array_element (`self.WorkLocations`)
    (if (`WorkLocationComponent.bIsEnabled` _array_element)
      (for _array_element_2 (`SceneComponent.GetChildrenComponents` _array_element false)
        (bind _asdecal_component (cast `DecalComponent` _array_element_2))
        (`SceneComponent.SetVisibility` _asdecal_component false false)))))

(fn `FindNearestAvailableWorkLocation`
  (params (NearestWorkLocationPosition :type "Vector Structure (by ref)") (WorkerPostion :type "Vector Structure"))
  (returns (FoundAvailable :type Boolean))
  (locals (ShortestDistance :type "Float (double-precision)") (FoundAvailableWorkLocation :type Boolean))
  (set `local.ShortestDistance` 1000000000.0)
  (set `local.FoundAvailableWorkLocation` false)
  (for _array_element (`self.WorkLocations`)
    (if (`WorkLocationComponent.bIsEnabled` _array_element)
      (if (not (`WorkLocationComponent.bIsOccupied` _array_element))
        (bind _returnvalue (`SceneComponent.K2_GetComponentLocation` _array_element))
        (bind _returnvalue_2 (`KismetMathLibrary.Vector_Distance` _returnvalue WorkerPostion))
        (if (< _returnvalue_2 (`local.ShortestDistance`))
          (set `local.ShortestDistance` _returnvalue_2)
          (`|VariableSetRef` NearestWorkLocationPosition _returnvalue)
          (set `local.FoundAvailableWorkLocation` true)))))
  (return (`local.FoundAvailableWorkLocation`)))

(fn `SetWorkLocationOccupied`
  (params (`Work Location Component` :type "PrimitiveComponent Object Reference") (IsOccupied :type Boolean))
  (bind _aswork_location_component (cast `WorkLocationComponent` `Work Location Component`))
  (set `WorkLocationComponent.bIsOccupied` IsOccupied _aswork_location_component))

(fn `UserConstructionScript`)