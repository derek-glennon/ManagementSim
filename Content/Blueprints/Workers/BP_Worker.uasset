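; Base worker character that is sent to work locations on work nodes and wears down their durability and skill bars.
; It moves via its AI controller, reroutes if the spot gets occupied, then snaps in facing the node.
; A looping timer, scaled by work speed and node difficulty, applies stat-versus-resistance strikes, updates progress bars and drives the tool animation.
; Active and ultimate abilities start on timer cooldowns, with empty hooks for child classes.
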(event `self.ReceiveBeginPlay`
  (set `self.MaxMoveSpeed` (`CharacterMovementComponent.MaxWalkSpeed` (`self.CharacterMovement`)))
  (bind _asbp_worker_aicontroller (cast `/Game/Blueprints/Workers/BP_WorkerAIController` (`self.GetController`)))
  (set `self.AIController` _asbp_worker_aicontroller)
  ;[1 0 0.8984] Abilities Start On Cooldown
  (bind _returnvalue (`KismetSystemLibrary.K2_SetTimer` null "OnActiveAbilityCooldownEnded" (`self.ActiveAbilityCooldownTime`))) ; Start Active Ability Cooldown
  (set `self.ActiveAbilityTimerHandle` _returnvalue)
  (bind _returnvalue_2 (`KismetSystemLibrary.K2_SetTimer` null "OnUltimateAbilityCooldownEnded" (`self.UltimateAbilityCooldownTime`))) ; Start Ultimate Ability Cooldown
  (set `self.UltimateAbilityTimerHandle` _returnvalue_2)
  (set `self.WorkerStats` (`self.BaseWorkerStats`)))

(event `self.ReceiveTick`
  (params (DeltaSeconds :type "Float (single-precision)"))
  (set `self.DeltaSeconds` DeltaSeconds)
  (switch `EPathFollowingStatus` (`AIController.GetMoveStatus` (`self.AIController`))
    (:`Idle`
      (if (`self.IsWorking`)
        (`self.HandlePerTickWorkingBehavior`)
        ;[0 0.927 1] Tool Animation While Working
        (if (`KismetSystemLibrary.K2_IsTimerPausedHandle` (`self.ProgressTimer`))
          (set `self.ToolAnimationValue` (`KismetSystemLibrary.K2_GetTimerElapsedTimeHandle` (`self.WorkProgressBarEmptyTimer`)))
          (else
            (set `self.ToolAnimationValue` (`KismetSystemLibrary.K2_GetTimerElapsedTimeHandle` (`self.ProgressTimer`)))))
        (bind _progresstime (`self.CalculateWorkProgressTime`))
        (bind (_direction _toolrotation) (`Timeline|Timeline` :`NewTime` (/ (`self.ToolAnimationValue`) _progresstime) :!via `SetNewTime`)
          (:`Update`
            (`SceneComponent.K2_SetRelativeRotation` (`self.Tool`) (`KismetMathLibrary.RotatorFromAxisAndAngle` (0.0 1.0 0.0) (* _toolrotation 360.0)) false false)))
        (else
          (`self.HandlePerTickNotWorkingBehavior`))))
    (:`Moving`
      (if (`WorkLocationComponent.bIsOccupied` (`self.GoalWorkLocation`))
        ;[1 0 0.007519] What to do if another worker reaches the same location as you before you get there
        (bind (_didfindnewgoal _newgoalworklocation) (`self.RecalculateGoalWorkLocation`))
        (if _didfindnewgoal
          (bind _output_get (set `self.GoalWorkLocation` _newgoalworklocation))
          (`self.MoveToGoalWorkLocation` (`self.GoalLocation`) (`self.GoalWorkNode`) _output_get)
          (else
            (`Controller.StopMovement` (`self.AIController`))
            (set `CharacterMovementComponent.MaxWalkSpeed` 0.0 (`self.CharacterMovement`)) ; For some reason if I don't zero this the workers will still slowly move
          ))
        (else
          ;[1 0 0.007519] What to check while moving towards a goal
          (bind _result (`self.HasReachedGoalLocation`))
          (if _result
            (`self.OnGoalLocationReached`)
            (if (`KismetSystemLibrary.DoesImplementInterface` (`self.GoalWorkNode`) "/Game/Blueprints/WorkNode/WorkLocations/BPI_WorkLocationActions.BPI_WorkLocationActions_C")
              (message `/Game/Blueprints/WorkNode/WorkLocations/BPI_WorkLocationActions.OnGoalWorkLocationReached` (`self.GoalWorkNode`) (`self.GoalWorkLocation`)))))))))

(event `/Game/Blueprints/Workers/BPI_UnitActions.MoveUnit`
  (params (GoalLocation :type "Vector Structure") (GoalWorkNode :type "/Game/Blueprints/WorkNode/BP_WorkNode Object Reference") (GoalWorkLocation :type "WorkLocationComponent Object Reference"))
  ;[0 0.1466 1] Goal Location Checks
  (`self.MoveToGoalWorkLocation` GoalLocation GoalWorkNode GoalWorkLocation))

(event `OnGoalLocationReached`
  ;[0 0.1466 1] Goal Location Checks
  (`self.OnReachedGoalLocation`))

(event `/Game/Blueprints/WorkNode/WorkLocations/BPI_WorkLocationActions.OnGoalWorkLocationLeft`
  ;[0 0.1466 1] Goal Location Checks
  (`self.OnLeftGoalLocation`))

(event `/Game/Blueprints/Workers/BPI_SelectionActions.Select`
  ;[0 0.1466 1] Selection Events
  (`SceneComponent.SetVisibility` (`self.SelectedArrow`) true false)
  (bind _asbp_work_progress_bar (cast `/Game/Blueprints/Workers/BP_WorkProgressBar` (`WidgetComponent.GetWidget` (`self.WorkProgressBar`))))
  (`Widget.SetVisibility` (`/Game/Blueprints/Workers/BP_WorkProgressBar.WorkProgressBar` _asbp_work_progress_bar) "SelfHitTestInvisible"))

(event `/Game/Blueprints/Workers/BPI_SelectionActions.Deselect`
  ;[0 0.1466 1] Selection Events
  (`SceneComponent.SetVisibility` (`self.SelectedArrow`) false false)
  (bind _asbp_work_progress_bar (cast `/Game/Blueprints/Workers/BP_WorkProgressBar` (`WidgetComponent.GetWidget` (`self.WorkProgressBar`))))
  (`Widget.SetVisibility` (`/Game/Blueprints/Workers/BP_WorkProgressBar.WorkProgressBar` _asbp_work_progress_bar) "Hidden"))

(event `/Game/Blueprints/WorkNode/BPI_WorkNodeActions.OnDurabilityBreakLimitReached`
  ;[0 0.927 1] Work Node is being destroyed because the durability break limit has been reached
  (`KismetSystemLibrary.K2_ClearAndInvalidateTimerHandle` (`self.ProgressTimer`))
  (set `self.IsWorking` false)
  (bind _asbp_work_progress_bar (cast `/Game/Blueprints/Workers/BP_WorkProgressBar` (`WidgetComponent.GetWidget` (`self.WorkProgressBar`))))
  (`/Game/Blueprints/Workers/BP_WorkProgressBar.SetWorkProgressBarPercent` _asbp_work_progress_bar 1.0)
  (message `/Game/Blueprints/Manager/HUD/WorkerHUDs/BPI_WorkerHUDActions.SetWorkProgressBarMini` (`self.WorkerHUD`) 1.0)
  (`SceneComponent.K2_SetRelativeRotation` :`self` (`self.Tool`)))

(event `/Game/Blueprints/Manager/HUD/WorkerHUDs/BPI_WorkerHUDActions.UseActiveAbility`
  ;[1 0 0.8984] Abilities
  (`self.OnActiveAbilityUsed`)
  (bind _returnvalue (`KismetSystemLibrary.K2_SetTimer` null "OnActiveAbilityCooldownEnded" (`self.ActiveAbilityCooldownTime`))) ; Start Active Ability Cooldown
  (set `self.ActiveAbilityTimerHandle` _returnvalue))

(event `/Game/Blueprints/Manager/HUD/WorkerHUDs/BPI_WorkerHUDActions.UseUltimateAbility`
  ;[1 0 0.8984] Abilities
  (`self.OnUltimateAbilityUsed`)
  (bind _returnvalue (`KismetSystemLibrary.K2_SetTimer` null "OnUltimateAbilityCooldownEnded" (`self.UltimateAbilityCooldownTime`))) ; Start Ultimate Ability Cooldown
  (set `self.UltimateAbilityTimerHandle` _returnvalue))

(fn `CalculateDurabilityDamage`
  (params (ProductivityPercent :type "Float (double-precision)" :default 1.0) (AdditionalDamage :type "Float (double-precision)"))
  (returns (DurabilityDamage :type "Float (double-precision)") (Progress :type "Float (double-precision)"))
  (bind (_durabilitybreaklimit _durabilitylimit _durabilityresistance) (break `/Game/Blueprints/WorkNode/FWorkNodeStats` (`/Game/Blueprints/WorkNode/BP_WorkNode.WorkNodeStats` (`self.GoalWorkNode`))))
  (bind _returnvalue (- (+ AdditionalDamage (* ProductivityPercent (`.Productivity_2_F2FDFBD94D0E511115BEC69335BE7442` (break `/Game/Blueprints/Workers/FWorkerStats` (`self.WorkerStats`))))) _durabilityresistance))
  (return (`KismetMathLibrary.FMax` _returnvalue) (`KismetMathLibrary.FMax` (/ _returnvalue _durabilitylimit))))

(fn `CalculateSkillDamage`
  (params (SkillPercent :type "Float (double-precision)" :default 1.0) (AdditionalDamage :type "Float (double-precision)"))
  (returns (SkillDamage :type "Float (double-precision)") (Progress :type "Float (double-precision)"))
  (bind (_durabilitybreaklimit _durabilitylimit _durabilityresistance _skilllimit _skillresistance) (break `/Game/Blueprints/WorkNode/FWorkNodeStats` (`/Game/Blueprints/WorkNode/BP_WorkNode.WorkNodeStats` (`self.GoalWorkNode`))))
  (bind _returnvalue (- (+ AdditionalDamage (* SkillPercent (`.Skill_4_70C134A240C624B7AC7CF6B9A785B90B` (break `/Game/Blueprints/Workers/FWorkerStats` (`self.WorkerStats`))))) _skillresistance))
  (return (`KismetMathLibrary.FMax` _returnvalue) (`KismetMathLibrary.FMax` (/ _returnvalue _skilllimit))))

(fn `CalculateWorkProgressTime`
  (returns (ProgressTime :type "Float (double-precision)"))
  (return (* (`.WorkSpeed_6_8203CFA6454ABA9D3441F583C7BECB88` (break `/Game/Blueprints/Workers/FWorkerStats` (`self.WorkerStats`))) (`.Difficulty_9_B97BDFC2452FE0EA63844FB0265E8AC5` (break `/Game/Blueprints/WorkNode/FWorkNodeStats` (`/Game/Blueprints/WorkNode/BP_WorkNode.WorkNodeStats` (`self.GoalWorkNode`)))))))

(fn `HandleDurabilityPerWorkerStrike`
  (locals (BPWorkProgressBar :type "/Game/Blueprints/Workers/BP_WorkProgressBar Object Reference") (DurabilityDamage :type "Float (double-precision)" :default 0.0) (NewDurabilityBarPercent :type "Float (double-precision)"))
  (bind _asbp_work_progress_bar (cast `/Game/Blueprints/Workers/BP_WorkProgressBar` (`WidgetComponent.GetWidget` (`self.WorkProgressBar`))))
  (set `local.BPWorkProgressBar` _asbp_work_progress_bar)
  (bind (_durabilitydamage _progress) (`self.CalculateDurabilityDamage` 1.0))
  (set `local.DurabilityDamage` _durabilitydamage)
  (bind _returnvalue (- (`/Game/Blueprints/Workers/BP_WorkProgressBar.GetWorkProgressBarPercent` (`local.BPWorkProgressBar`)) _progress))
  (if (< _returnvalue 0.0)
    (set `local.NewDurabilityBarPercent` 0.0)
    (else
      (set `local.NewDurabilityBarPercent` _returnvalue)))
  (if (`KismetMathLibrary.NearlyEqual_FloatFloat` (`local.NewDurabilityBarPercent`))
    ;[1 1 1] When Progress Bar Reaches 0
    (`/Game/Blueprints/Workers/BP_WorkProgressBar.SetWorkProgressBarPercent` (`local.BPWorkProgressBar`) 0.0)
    (message `/Game/Blueprints/Manager/HUD/WorkerHUDs/BPI_WorkerHUDActions.SetWorkProgressBarMini` (`self.WorkerHUD`) 0.0)
    (bind _progresstime (`self.CalculateWorkProgressTime`))
    (bind _returnvalue_2 (`KismetSystemLibrary.K2_SetTimer` null "OnWorkProgressBarEmpty" _progresstime)) ; Set a slight delay before starting work again
    (set `self.WorkProgressBarEmptyTimer` _returnvalue_2)
    (message `/Game/Blueprints/WorkNode/BPI_WorkNodeActions.OnDurabilityBroken` (`self.GoalWorkNode`))
    (`KismetSystemLibrary.K2_PauseTimerHandle` (`self.ProgressTimer`))
    (return)
    (else
      ;[1 1 1] Decrease Progress Bar
      (`/Game/Blueprints/Workers/BP_WorkProgressBar.SetWorkProgressBarPercent` (`local.BPWorkProgressBar`) (`local.NewDurabilityBarPercent`))
      (message `/Game/Blueprints/Manager/HUD/WorkerHUDs/BPI_WorkerHUDActions.SetWorkProgressBarMini` (`self.WorkerHUD`) (`local.NewDurabilityBarPercent`))
      (if (`KismetSystemLibrary.DoesImplementInterface` (`self.GoalWorkNode`) "/Game/Blueprints/WorkNode/BPI_WorkNodeActions.BPI_WorkNodeActions_C")
        (message `/Game/Blueprints/WorkNode/BPI_WorkNodeActions.DurabilityDamageDealtToNode` (`self.GoalWorkNode`) (`local.DurabilityDamage`))
        (return)))))

(fn `HandlePerTickNotWorkingBehavior`
  ;[1 1 1] For children to perform specific actions per tick while the worker is not working
  (return))

(fn `HandlePerTickWorkingBehavior`
  ;[1 1 1] For children to before specific behavior per tick while working
  (return))

(fn `HandleSkillPerWorkerStrike`
  (locals (BPSkillBreakBar :type "/Game/Blueprints/WorkNode/BP_WorkNodeUI Object Reference") (SkillDamage :type "Float (double-precision)") (NewSkillBarPercent :type "Float (double-precision)"))
  (`/Engine/EditorBlueprintResources/StandardMacros.IsValid` (`self.GoalWorkNode`)
    (:`Is Valid`
      (if (not (`KismetSystemLibrary.K2_IsValidTimerHandle` (`/Game/Blueprints/WorkNode/BP_WorkNode.SkillBarRechargingTimer` (`self.GoalWorkNode`))))
        (bind _asbp_work_node_ui (cast `/Game/Blueprints/WorkNode/BP_WorkNodeUI` (`WidgetComponent.GetWidget` (`/Game/Blueprints/WorkNode/BP_WorkNode.UIWidget` (`self.GoalWorkNode`)))))
        (set `local.BPSkillBreakBar` _asbp_work_node_ui)
        (bind (_skilldamage _progress) (`self.CalculateSkillDamage` 1.0))
        (set `local.SkillDamage` _skilldamage)
        (bind _returnvalue (- (`/Game/Blueprints/WorkNode/BP_WorkNodeUI.SkillBreakBarPercent` (`local.BPSkillBreakBar`)) _progress))
        (if (< _returnvalue 0.0)
          (set `local.NewSkillBarPercent` 0.0)
          (else
            (set `local.NewSkillBarPercent` _returnvalue)))
        (if (`KismetMathLibrary.NearlyEqual_FloatFloat` (`local.NewSkillBarPercent`))
          ;[1 1 1] Skill Bar Broken
          (set `/Game/Blueprints/WorkNode/BP_WorkNodeUI.SkillBreakBarPercent` 0.0 (`local.BPSkillBreakBar`))
          (message `/Game/Blueprints/WorkNode/BPI_WorkNodeActions.OnSkillBroken` (`self.GoalWorkNode`))
          (return)
          (else
            ;[1 1 1] Skill Damage Dealt To Node
            (set `/Game/Blueprints/WorkNode/BP_WorkNodeUI.SkillBreakBarPercent` (`local.NewSkillBarPercent`) (`local.BPSkillBreakBar`))
            (message `/Game/Blueprints/WorkNode/BPI_WorkNodeActions.SkillDamageDealtToNode` (`self.GoalWorkNode`) (`local.SkillDamage`))
            (return)))
        (else
          (return))))
    (:`Is Not Valid`
      (return))))

(fn `HasReachedGoalLocation`
  (returns (result :type Boolean))
  (return (<= (`KismetMathLibrary.Vector_Distance` (`self.K2_GetActorLocation`) (`self.GoalLocation`)) (`self.GoalPositionSnapDistance`))))

(fn `MoveToGoalWorkLocation`
  (params (GoalLocation :type "Vector Structure") (GoalWorkNode :type "/Game/Blueprints/WorkNode/BP_WorkNode Object Reference") (GoalWorkLocation :type "WorkLocationComponent Object Reference"))
  (set `self.GoalWorkNode` GoalWorkNode)
  (bind _output_get (set `self.GoalLocation` GoalLocation))
  (set `self.GoalWorkLocation` GoalWorkLocation)
  (set `CharacterMovementComponent.MaxWalkSpeed` (`self.MaxMoveSpeed`) (`self.CharacterMovement`))
  (`AIController.MoveToLocation` (`self.AIController`) _output_get 1.0 false true false true null false)
  (`self.SetCanAffectNavigationGeneration` self false false))

(fn `OnActiveAbilityCooldownEnded`
  (`KismetSystemLibrary.K2_ClearAndInvalidateTimerHandle` (`self.ActiveAbilityTimerHandle`)))

(fn `OnActiveAbilityUsed`
  ;[1 1 1] Children Can Override
  (return))

(fn `OnLeftGoalLocation`
  ;[0 0.927 1] Set work variables on Goal Left
  (set `self.IsWorking` false)
  (`SceneComponent.SetVisibility` (`self.WorkProgressBar`) false false)
  (`KismetSystemLibrary.K2_ClearAndInvalidateTimerHandle` (`self.ProgressTimer`)))

(fn `OnReachedGoalLocation`
  ;[1 0 0.007519] Set Navigation Variables on Goal Reached
  (`Controller.StopMovement` (`self.AIController`))
  (set `CharacterMovementComponent.MaxWalkSpeed` 0.0 (`self.CharacterMovement`))
  (`self.K2_SetActorLocationAndRotation` (`self.GoalLocation`) (`KismetMathLibrary.FindLookAtRotation` (`self.GoalLocation`) (`self.K2_GetActorLocation` (`self.GoalWorkNode`)))) ; Snap to Goal Location and Rotation
  (`self.SetCanAffectNavigationGeneration` self true false)
  ;[0 0.927 1] Set Work Variables on Goal Reached
  (set `self.IsWorking` true)
  (`SceneComponent.SetVisibility` (`self.WorkProgressBar`) true false)
  (bind _asbp_work_progress_bar (cast `/Game/Blueprints/Workers/BP_WorkProgressBar` (`WidgetComponent.GetWidget` (`self.WorkProgressBar`))))
  (`/Game/Blueprints/Workers/BP_WorkProgressBar.SetWorkProgressBarPercent` _asbp_work_progress_bar 1.0)
  (message `/Game/Blueprints/Manager/HUD/WorkerHUDs/BPI_WorkerHUDActions.SetWorkProgressBarMini` (`self.WorkerHUD`) 1.0)
  (bind _progresstime (`self.CalculateWorkProgressTime`))
  (bind _returnvalue (`KismetSystemLibrary.K2_SetTimer` null "UpdateWorkProgress" _progresstime true))
  (set `self.ProgressTimer` _returnvalue))

(fn `OnUltimateAbilityCooldownEnded`
  (`KismetSystemLibrary.K2_ClearAndInvalidateTimerHandle` (`self.UltimateAbilityTimerHandle`)))

(fn `OnUltimateAbilityUsed`
  ;[1 1 1] Child Can Override
  (return))

(fn `OnWorkProgressBarEmpty`
  (`KismetSystemLibrary.K2_ClearAndInvalidateTimerHandle` (`self.WorkProgressBarEmptyTimer`))
  (bind _asbp_work_progress_bar (cast `/Game/Blueprints/Workers/BP_WorkProgressBar` (`WidgetComponent.GetWidget` (`self.WorkProgressBar`))))
  (`/Game/Blueprints/Workers/BP_WorkProgressBar.SetWorkProgressBarPercent` _asbp_work_progress_bar 1.0)
  (message `/Game/Blueprints/Manager/HUD/WorkerHUDs/BPI_WorkerHUDActions.SetWorkProgressBarMini` (`self.WorkerHUD`) 1.0)
  (`KismetSystemLibrary.K2_UnPauseTimerHandle` (`self.ProgressTimer`))
  (if (`KismetSystemLibrary.DoesImplementInterface` (`self.GoalWorkNode`) "/Game/Blueprints/WorkNode/BPI_WorkNodeActions.BPI_WorkNodeActions_C")
    _))

(fn `RecalculateGoalWorkLocation`
  (returns (DidFindNewGoal :type Boolean) (NewGoalWorkLocation :type "WorkLocationComponent Object Reference"))
  (bind (_foundavailable _goalworklocation) (`/Game/Blueprints/WorkNode/BP_WorkNode.FindNearestAvailableWorkLocation` (`self.GoalWorkNode`) (`self.GoalLocation`) (`self.K2_GetActorLocation`)))
  (return _foundavailable _goalworklocation))

(fn `UpdateWorkProgress`
  (`/Engine/EditorBlueprintResources/StandardMacros.IsValid` (`self.GoalWorkNode`)
    (:`Is Valid`
      (`self.HandleDurabilityPerWorkerStrike`)
      (`self.HandleSkillPerWorkerStrike`))))

(fn `UserConstructionScript`)