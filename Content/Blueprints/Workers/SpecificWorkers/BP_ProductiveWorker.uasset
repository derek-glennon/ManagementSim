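; Productive worker subclass that defines this worker type's passive, auto, active and ultimate abilities by overriding parent work hooks.
; Passive rolls an extra durability strike, with odds depending on skill bar recharge; auto sets durability and skill damage percentages.
; Active scales WorkSpeed for a few counted strikes, restarting the looping progress timer on change.
; Ultimate boosts the next strike and briefly raises move speed; both are usable only while working.
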(fn `CalculateDurabilityDamage`
  (params (ProductivityPercent :type "Float (double-precision)") (AdditionalDamage :type "Float (double-precision)"))
  (returns (DurabilityDamage :type "Float (double-precision)") (Progress :type "Float (double-precision)"))
  (locals (UltimateDamage :type "Float (double-precision)"))
  ;[1 0 0.8984] Ultimate Ability: Additional 150% Damage to next Strike
  (if (`self.ShouldNextStrikeDealsUltimateDamage`)
    (set `local.UltimateDamage` (* (`.Productivity_2_F2FDFBD94D0E511115BEC69335BE7442` (break `/Game/Blueprints/Workers/FWorkerStats` (`self.WorkerStats`))) 1.5))
    (set `self.ShouldNextStrikeDealsUltimateDamage` false)
    (else
      (set `local.UltimateDamage` 0.0)))
  ;[1 0 0.8984] Auto Ability: 50% of Productivity
  (bind (_durabilitydamage _progress) (`parent.CalculateDurabilityDamage` 0.5 (`local.UltimateDamage`)))
  (return _durabilitydamage _progress))

(fn `CalculateSkillDamage`
  (params (SkillPercent :type "Float (double-precision)") (AdditionalDamage :type "Float (double-precision)"))
  (returns (SkillDamage :type "Float (double-precision)") (Progress :type "Float (double-precision)"))
  ;[1 0 0.8984] Auto Ability: 20% Skill
  (bind (_skilldamage _progress) (`parent.CalculateSkillDamage` 0.2 0.0))
  (return _skilldamage _progress))

(fn `HandleDurabilityPerWorkerStrike`
  (bind (_productivity _skill _workspeed _movespeed) (break `/Game/Blueprints/Workers/FWorkerStats` (`self.WorkerStats`)))
  (bind (_productivity_2 _skill_2 _workspeed_2 _movespeed_2) (break `/Game/Blueprints/Workers/FWorkerStats` (`self.WorkerStats`)))
  (`parent.HandleDurabilityPerWorkerStrike`)
  (if (!= (`self.WorkSpeedIncreaseCounter`) 0)
    (if (== (`self.WorkSpeedIncreaseCounter`) 4)
      ;[1 0 0.8984] Active Ability: Set New Work Speed
      (if (`KismetSystemLibrary.K2_IsValidTimerHandle` (`/Game/Blueprints/WorkNode/BP_WorkNode.SkillBarRechargingTimer` (`self.GoalWorkNode`)))
        (set `self.WorkSpeedIncreasePercent` 0.4)
        (else
          (set `self.WorkSpeedIncreasePercent` 0.6)))
      (set `self.WorkerStats` (make `/Game/Blueprints/Workers/FWorkerStats` _productivity _skill (* _workspeed (`self.WorkSpeedIncreasePercent`)) _movespeed))
      (`/Engine/EditorBlueprintResources/StandardMacros.DecrementInt` (`self.WorkSpeedIncreaseCounter`)
        (:`  `
          ;[1 1 1] Start New Work Progress Timer With Buff
          (`KismetSystemLibrary.K2_ClearAndInvalidateTimerHandle` (`self.ProgressTimer`))
          (bind _progresstime (`self.CalculateWorkProgressTime`))
          (bind _returnvalue (`KismetSystemLibrary.K2_SetTimer` null "UpdateWorkProgress" _progresstime true))
          (set `self.ProgressTimer` _returnvalue)))
      (else
        ;[1 0 0.8984] Active Ability: Work Speed Increase Only Lasts For 4 Strikes
        (`/Engine/EditorBlueprintResources/StandardMacros.DecrementInt` (`self.WorkSpeedIncreaseCounter`)
          (:`  `
            (if (== (`self.WorkSpeedIncreaseCounter`) 0)
              (set `self.WorkerStats` (make `/Game/Blueprints/Workers/FWorkerStats` _productivity_2 _skill_2 (/ _workspeed_2 (`self.WorkSpeedIncreasePercent`)) _movespeed_2))
              ;[1 1 1] Restart Work Progress Timer without buff
              (`KismetSystemLibrary.K2_ClearAndInvalidateTimerHandle` (`self.ProgressTimer`))
              (bind _progresstime_2 (`self.CalculateWorkProgressTime`))
              (bind _returnvalue_2 (`KismetSystemLibrary.K2_SetTimer` null "UpdateWorkProgress" _progresstime_2 true))
              (set `self.ProgressTimer` _returnvalue_2))))))))

(fn `HandlePerTickNotWorkingBehavior`
  ;[1 1 1] Active Ability can only be used while working
  (if (`self.IsActiveAbilityUsable`)
    (set `self.IsActiveAbilityUsable` false))
  ;[1 1 1] Ultimate Ability Can only be used while working
  (if (`self.IsUltimateAbilityUsable`)
    (set `self.IsUltimateAbilityUsable` false))
  (return))

(fn `HandlePerTickWorkingBehavior`
  ;[1 1 1] Active Ability can only be used while working
  (if (not (`self.IsActiveAbilityUsable`))
    (set `self.IsActiveAbilityUsable` true))
  ;[1 1 1] Ultimate Ability Can only be used while working
  (if (not (`self.IsUltimateAbilityUsable`))
    (set `self.IsUltimateAbilityUsable` true))
  (return))

(fn `OnActiveAbilityUsed`
  ;[1 0 0.8984] Active Ability: Increase Work Speed by 40% for next 4 strikes. If skill bar is broken when activated, increase by an additional 20%
  (set `self.WorkSpeedIncreaseCounter` 4))

(fn `OnUltimateAbilityMoveSpeedBuffOver`
  (`KismetSystemLibrary.K2_ClearAndInvalidateTimerHandle` (`self.UltimateMoveSpeedBuffTimer`))
  (set `self.MaxMoveSpeed` (/ (`self.MaxMoveSpeed`) 1.5)))

(fn `OnUltimateAbilityUsed`
  ;[1 0 0.8984] Ultimate Ability: Deal Additional Damage Next Strike and Increase Movement Speed for 5 sec
  (set `self.ShouldNextStrikeDealsUltimateDamage` true)
  (bind _returnvalue (`KismetSystemLibrary.K2_SetTimer` null "OnUltimateAbilityMoveSpeedBuffOver" 5.0))
  (set `self.UltimateMoveSpeedBuffTimer` _returnvalue)
  (set `self.MaxMoveSpeed` (* 1.5 (`self.MaxMoveSpeed`))))

(fn `UpdateWorkProgress`
  (locals (DoubleStrikePercent :type "Float (double-precision)"))
  (`parent.UpdateWorkProgress`)
  (`/Engine/EditorBlueprintResources/StandardMacros.IsValid` (`self.GoalWorkNode`)
    (:`Is Valid`
      ;[1 0 0.8984] Passive Ability: 10% Chance to Strike Twice, Doubles when the skill bar is broken
      (if (`KismetSystemLibrary.K2_IsValidTimerHandle` (`/Game/Blueprints/WorkNode/BP_WorkNode.SkillBarRechargingTimer` (`self.GoalWorkNode`)))
        (set `local.DoubleStrikePercent` 0.2)
        (else
          (set `local.DoubleStrikePercent` 0.1)))
      (if (<= (`KismetMathLibrary.RandomFloat`) (`local.DoubleStrikePercent`))
        (`self.HandleDurabilityPerWorkerStrike`)))))

(fn `UserConstructionScript`
  (`parent.UserConstructionScript`))