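; BP_SkillfulWorker is a specific worker type whose active and ultimate abilities are usable only while it is working.
; It implements the per-tick working and not-working behavior functions to switch both ability-usable flags on and off, writing each only when it needs to change.
; The event graph holds only disabled stub events, and the construction script just calls the parent.
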(fn `HandlePerTickNotWorkingBehavior`
  ;[1 1 1] Active Ability can only be used while working
  (if (`self.IsActiveAbilityUsable`)
    (set `self.IsActiveAbilityUsable` false))
  ;[1 1 1] Ultimate Ability Can only be used while working
  (if (`self.IsUltimateAbilityUsable`)
    (set `self.IsUltimateAbilityUsable` false))
  (return))

(fn `HandlePerTickWorkingBehavior`
  ;[1 1 1] Active Ability can only be used while working
  (if (not (`self.IsActiveAbilityUsable`))
    (set `self.IsActiveAbilityUsable` true))
  ;[1 1 1] Ultimate Ability Can only be used while working
  (if (not (`self.IsUltimateAbilityUsable`))
    (set `self.IsUltimateAbilityUsable` true))
  (return))

(fn `UserConstructionScript`
  (`parent.UserConstructionScript`))