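; Harvestable work node actor where workers occupy work locations and break durability and skill bars to make it drop loot.
; Overlap and goal-reached events track occupancy, a nearest-free-spot search serves workers, and cursor hover reveals free-spot decals.
; Durability breaks launch item drops; at the break limit it notifies the first occupying worker and destroys itself.
; Skill breaks apply a timed condition that recomputes stats from base, lowering resistance and boosting drops until recharged.
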(event `self.ReceiveBeginPlay`
  (add `self.OnBeginCursorOver` (`|CreateDelegate` :!event `OnBeginCursorOver_Event`))
  (add `self.OnEndCursorOver` (`|CreateDelegate` :!event `OnEndCursorOver_Event`))
  (set `self.WorkNodeStats` (`self.BaseWorkNodeStats`))
  (bind _asbp_work_node_ui (cast `/Game/Blueprints/WorkNode/BP_WorkNodeUI` (`WidgetComponent.GetWidget` (`self.UIWidget`))))
  (`TextBlock.SetText` (`/Game/Blueprints/WorkNode/BP_WorkNodeUI.DurabilityBreakLimitCounterText` _asbp_work_node_ui) (`KismetTextLibrary.Conv_IntToText` (`.DurabilityBreakLimit_2_FD8371F644139CC31ACE70A8194295A5` (break `/Game/Blueprints/WorkNode/FWorkNodeStats` (`self.BaseWorkNodeStats`)))))
  ;[1 0 0.003032] Create Work Locations Array
  (for _array_element (`self.K2_GetComponentsByClass` "/Script/ManagementSim.WorkLocationComponent")
    (if (`WorkLocationComponent.bIsEnabled` _array_element)
      (`KismetArrayLibrary.Array_Add` (`self.WorkLocations`) _array_element))))

(event `/Game/Blueprints/WorkNode/BPI_WorkNodeActions.DurabilityDamageDealtToNode`
  (params (Damage :type "Float (double-precision)"))
  ;[1 0.1224 0.05274] Handle Durability Damage
  (bind _returnvalue (`|CreateWidget` "/Game/Blueprints/WorkNode/DamageNumbers/BP_DamageNumber.BP_DamageNumber_C" null Damage self))
  (`UserWidget.AddToViewport` _returnvalue 0))

(event `/Game/Blueprints/WorkNode/BPI_WorkNodeActions.SkillDamageDealtToNode`
  (params (Damage :type "Float (double-precision)"))
  ;[0.01873 0.1371 1] Handle Skill Damage
  (bind _returnvalue (`|CreateWidget` "/Game/Blueprints/WorkNode/DamageNumbers/BP_DamageNumber.BP_DamageNumber_C" null Damage self "NewEnumerator1"))
  (`UserWidget.AddToViewport` _returnvalue 0))

(event `/Game/Blueprints/WorkNode/BPI_WorkNodeActions.OnDurabilityBroken`
  ;[1 0.1224 0.05274] Handle Durability Bar Broken
  (`self.HandleDurabilityBarBroken`))

(event `/Game/Blueprints/WorkNode/BPI_WorkNodeActions.OnSkillBroken`
  ;[0.01873 0.1371 1] Handle Skill Bar Broken
  (`self.HandleSkillBarBroken`))

(event `self.ReceiveTick`
  (params (DeltaSeconds :type "Float (single-precision)"))
  ;[0.01873 0.1371 1] Skill Bar Recharge
  (if (`KismetSystemLibrary.K2_IsValidTimerHandle` (`self.SkillBarRechargingTimer`))
    (bind _asbp_work_node_ui (cast `/Game/Blueprints/WorkNode/BP_WorkNodeUI` (`WidgetComponent.GetWidget` (`self.UIWidget`))))
    (set `/Game/Blueprints/WorkNode/BP_WorkNodeUI.SkillBreakBarPercent` (/ (`KismetSystemLibrary.K2_GetTimerElapsedTimeHandle` (`self.SkillBarRechargingTimer`)) (`.SkillBarRechargeTime_18_69E5B356458FDB957B0C19BCDDD3BADF` (break `/Game/Blueprints/WorkNode/FWorkNodeStats` (`self.WorkNodeStats`)))) _asbp_work_node_ui)))

(event `self.WorkLocation0.OnComponentBeginOverlap`
  (params (OverlappedComponent :type "PrimitiveComponent Object Reference") (OtherActor :type "Actor Object Reference") (OtherComp :type "PrimitiveComponent Object Reference") (OtherBodyIndex :type Integer) (bFromSweep :type Boolean) (SweepResult :type "HitResult Structure (by ref)"))
  ;[0 0.1048 1] Begin Overlap
  (`self.HandleWorkLocationOverlapBegin` OverlappedComponent OtherActor))

(event `/Game/Blueprints/WorkNode/WorkLocations/BPI_WorkLocationActions.OnGoalWorkLocationReached`
  (params (WorkLocation :type "WorkLocationComponent Object Reference"))
  (bind _returnvalue (`KismetArrayLibrary.Array_Find` (`self.WorkLocations`) WorkLocation))
  (bind _output (`|GetArrayItem` (`self.WorkLocations`) _returnvalue))
  ;[1 0.3188 0] A Worker reached their Goal Work Location
  (if (!= _returnvalue -1)
    (set `WorkLocationComponent.bIsOccupied` true _output)
    (`KismetArrayLibrary.Array_Set` (`self.WorkLocations`) _returnvalue _output)))

(event `self.WorkLocation1.OnComponentBeginOverlap`
  (params (OverlappedComponent :type "PrimitiveComponent Object Reference") (OtherActor :type "Actor Object Reference") (OtherComp :type "PrimitiveComponent Object Reference") (OtherBodyIndex :type Integer) (bFromSweep :type Boolean) (SweepResult :type "HitResult Structure (by ref)"))
  ;[0 0.1048 1] Begin Overlap
  (`self.HandleWorkLocationOverlapBegin` OverlappedComponent OtherActor))

(event `self.WorkLocation2.OnComponentBeginOverlap`
  (params (OverlappedComponent :type "PrimitiveComponent Object Reference") (OtherActor :type "Actor Object Reference") (OtherComp :type "PrimitiveComponent Object Reference") (OtherBodyIndex :type Integer) (bFromSweep :type Boolean) (SweepResult :type "HitResult Structure (by ref)"))
  ;[0 0.1048 1] Begin Overlap
  (`self.HandleWorkLocationOverlapBegin` OverlappedComponent OtherActor))

(event `self.WorkLocation3.OnComponentBeginOverlap`
  (params (OverlappedComponent :type "PrimitiveComponent Object Reference") (OtherActor :type "Actor Object Reference") (OtherComp :type "PrimitiveComponent Object Reference") (OtherBodyIndex :type Integer) (bFromSweep :type Boolean) (SweepResult :type "HitResult Structure (by ref)"))
  ;[0 0.1048 1] Begin Overlap
  (`self.HandleWorkLocationOverlapBegin` OverlappedComponent OtherActor))

(event `self.WorkLocation0.OnComponentEndOverlap`
  (params (OverlappedComponent :type "PrimitiveComponent Object Reference") (OtherActor :type "Actor Object Reference") (OtherComp :type "PrimitiveComponent Object Reference") (OtherBodyIndex :type Integer))
  ;[0 0.1048 1] End Overlap
  (`self.HandleWorkLocationOverlapEnd` OverlappedComponent OtherActor))

(event `self.WorkLocation1.OnComponentEndOverlap`
  (params (OverlappedComponent :type "PrimitiveComponent Object Reference") (OtherActor :type "Actor Object Reference") (OtherComp :type "PrimitiveComponent Object Reference") (OtherBodyIndex :type Integer))
  ;[0 0.1048 1] End Overlap
  (`self.HandleWorkLocationOverlapEnd` OverlappedComponent OtherActor))

(event `self.WorkLocation2.OnComponentEndOverlap`
  (params (OverlappedComponent :type "PrimitiveComponent Object Reference") (OtherActor :type "Actor Object Reference") (OtherComp :type "PrimitiveComponent Object Reference") (OtherBodyIndex :type Integer))
  ;[0 0.1048 1] End Overlap
  (`self.HandleWorkLocationOverlapEnd` OverlappedComponent OtherActor))

(event `self.WorkLocation3.OnComponentEndOverlap`
  (params (OverlappedComponent :type "PrimitiveComponent Object Reference") (OtherActor :type "Actor Object Reference") (OtherComp :type "PrimitiveComponent Object Reference") (OtherBodyIndex :type Integer))
  ;[0 0.1048 1] End Overlap
  (`self.HandleWorkLocationOverlapEnd` OverlappedComponent OtherActor))

(event `OnBeginCursorOver_Event` :!signature `self.OnBeginCursorOver`
  (params (TouchedActor :type "Actor Object Reference"))
  ;[0 0.1048 1] Set Visibility of UI Elements On Cursor Over
  (for _array_element (`self.WorkLocations`)
    (if (`WorkLocationComponent.bIsEnabled` _array_element)
      (if (not (`WorkLocationComponent.bIsOccupied` _array_element))
        (for _array_element_2 (`SceneComponent.GetChildrenComponents` _array_element false)
          (bind _asdecal_component (cast `DecalComponent` _array_element_2))
          (`SceneComponent.SetVisibility` _asdecal_component true false))))))

(event `OnEndCursorOver_Event` :!signature `self.OnEndCursorOver`
  (params (TouchedActor :type "Actor Object Reference"))
  ;[0 0.1048 1] Set Visibility of UI Elements On Cursor Over
  (for _array_element (`self.WorkLocations`)
    (if (`WorkLocationComponent.bIsEnabled` _array_element)
      (for _array_element_2 (`SceneComponent.GetChildrenComponents` _array_element false)
        (bind _asdecal_component (cast `DecalComponent` _array_element_2))
        (`SceneComponent.SetVisibility` _asdecal_component false false)))))

(fn `DropItem`
  (params (Item :type "/Game/Blueprints/Items/BP_Item Class Reference"))
  (bind _returnvalue (`|SpawnActorFromClass` Item (`KismetMathLibrary.MakeTransform` (+ (.location (`self.GetTransform`)) (0.0 0.0 100.0)) (`KismetMathLibrary.RandomRotator` false) (`.StaticMeshDefaultScale` (defaults `Object` Item))) "Undefined" "OverrideRootScale" null null))
  (`PrimitiveComponent.AddForce` (`/Game/Blueprints/Items/BP_Item.PickupMesh` _returnvalue) (`KismetMathLibrary.MakeVector` (`KismetMathLibrary.RandomFloatInRange` -15000.0 15000.0) (`KismetMathLibrary.RandomFloatInRange` -15000.0 15000.0) (`KismetMathLibrary.RandomFloatInRange` 20000.0 30000.0)) "None" false)
  (return))

(fn `FindNearestAvailableWorkLocation`
  (params (NearestWorkLocationPosition :type "Vector Structure (by ref)") (WorkerPostion :type "Vector Structure"))
  (returns (FoundAvailable :type Boolean) (GoalWorkLocation :type "WorkLocationComponent Object Reference"))
  (locals (ShortestDistance :type "Float (double-precision)") (FoundAvailableWorkLocation :type Boolean) (NearestWorkLocation :type "WorkLocationComponent Object Reference"))
  (set `local.ShortestDistance` 1000000000.0)
  (set `local.FoundAvailableWorkLocation` false)
  (for _array_element (`self.WorkLocations`)
    (if (`WorkLocationComponent.bIsEnabled` _array_element)
      (if (not (`WorkLocationComponent.bIsOccupied` _array_element))
        (bind _returnvalue (`SceneComponent.K2_GetComponentLocation` _array_element))
        (bind _returnvalue_2 (`KismetMathLibrary.Vector_Distance` _returnvalue WorkerPostion))
        (if (< _returnvalue_2 (`local.ShortestDistance`))
          (set `local.ShortestDistance` _returnvalue_2)
          (`|VariableSetRef` NearestWorkLocationPosition _returnvalue)
          (set `local.FoundAvailableWorkLocation` true)
          (set `local.NearestWorkLocation` _array_element)))))
  (return (`local.FoundAvailableWorkLocation`) (`local.NearestWorkLocation`)))

(fn `HandleDurabilityBarBroken`
  (for _ (range (`.ItemDropAmount_21_8017640844CDC45DF7861CB8166C8EFA` (break `/Game/Blueprints/WorkNode/FWorkNodeStats` (`self.WorkNodeStats`))))
    ;[0.9881 1 0.04085] Drop Items
    (`/Game/Blueprints/Items/BP_ItemLootTable.SetItemToDrop` (`self.ItemLootTable`))
    (`self.DropItem` (`/Game/Blueprints/Items/BP_ItemLootTable.ItemToDrop` (`self.ItemLootTable`))))
  (bind _result (`/Engine/EditorBlueprintResources/StandardMacros.IncrementInt` (`self.CurrentDurabilityBreak`))
    (:`  `
      (if (>= _result (`.DurabilityBreakLimit_2_FD8371F644139CC31ACE70A8194295A5` (break `/Game/Blueprints/WorkNode/FWorkNodeStats` (`self.WorkNodeStats`))))
        ;[1 1 1] Let the Workers know their Work Node is being destroyed
        (for _array_element (`self.WorkLocations`)
          (if (`WorkLocationComponent.bIsOccupied` _array_element)
            (bind _workercharacter (`WorkLocationComponent.WorkerCharacter` _array_element))
            (if (`KismetSystemLibrary.DoesImplementInterface` _workercharacter "/Game/Blueprints/WorkNode/BPI_WorkNodeActions.BPI_WorkNodeActions_C")
              (message `/Game/Blueprints/WorkNode/BPI_WorkNodeActions.OnDurabilityBreakLimitReached` _workercharacter)
              (`self.K2_DestroyActor`)
              (return))))
        (else
          (bind _asbp_work_node_ui (cast `/Game/Blueprints/WorkNode/BP_WorkNodeUI` (`WidgetComponent.GetWidget` (`self.UIWidget`))))
          (`TextBlock.SetText` (`/Game/Blueprints/WorkNode/BP_WorkNodeUI.DurabilityBreakLimitCounterText` _asbp_work_node_ui) (`KismetTextLibrary.Conv_IntToText` (- (`.DurabilityBreakLimit_2_FD8371F644139CC31ACE70A8194295A5` (break `/Game/Blueprints/WorkNode/FWorkNodeStats` (`self.BaseWorkNodeStats`))) (`self.CurrentDurabilityBreak`))))
          (return))))))

(fn `HandleSkillBarBroken`
  (bind _returnvalue (`KismetSystemLibrary.K2_SetTimer` null "SkillBarDoneRecharging" (`.SkillBarRechargeTime_18_69E5B356458FDB957B0C19BCDDD3BADF` (break `/Game/Blueprints/WorkNode/FWorkNodeStats` (`self.WorkNodeStats`)))))
  (set `self.SkillBarRechargingTimer` _returnvalue)
  ;[0.1281 0.2865 0.2779] Apply Conditions
  (`BlueprintMapLibrary.Map_Add` (`self.WorkNodeConditions`) "NewEnumerator0" 1)
  (bind _newworknodestats (`self.ModifyStatsBasedOnConditions` (`self.BaseWorkNodeStats`) (`self.WorkNodeConditions`)))
  (set `self.WorkNodeStats` _newworknodestats))

(fn `HandleWorkLocationOverlapBegin`
  (params (`Work Location Component` :type "PrimitiveComponent Object Reference") (OtherActor :type "Actor Object Reference"))
  ;[1 1 1] Is a Worker Overlapping a Work Location?
  (bind _aswork_location_component (cast `WorkLocationComponent` `Work Location Component`))
  (bind _asworker_character (cast `WorkerCharacter` OtherActor))
  ;[1 1 1] If a Work Location doesn't currently have a Worker on it, assign this Worker to it
  (if (`WorkLocationComponent.bIsEnabled` _aswork_location_component)
    (if (not (`WorkLocationComponent.bIsOccupied` _aswork_location_component))
      (set `WorkLocationComponent.WorkerCharacter` _asworker_character _aswork_location_component))))

(fn `HandleWorkLocationOverlapEnd`
  (params (`Work Location Component` :type "PrimitiveComponent Object Reference") (OtherActor :type "Actor Object Reference"))
  ;[1 1 1] Is a Worker Overlapping a Work Location?
  (bind _aswork_location_component (cast `WorkLocationComponent` `Work Location Component`))
  (bind _asworker_character (cast `WorkerCharacter` OtherActor))
  ;[1 1 1] Check if the Worker leaving is the one assigned to the Work Location
  (if (== (`WorkLocationComponent.WorkerCharacter` _aswork_location_component) _asworker_character)
    (set `WorkLocationComponent.bIsOccupied` false _aswork_location_component)
    ;[1 1 1] Tell the Worker they have left their previous work location
    (message `/Game/Blueprints/WorkNode/WorkLocations/BPI_WorkLocationActions.OnGoalWorkLocationLeft` _asworker_character)))

(fn `ModifyStatsBasedOnConditions`
  (params (WorkNodeStats :type "/Game/Blueprints/WorkNode/FWorkNodeStats Structure") (WorkNodeConditions :type "Map of /Game/Blueprints/WorkNode/EWorkNodeConditions Enum to Integer"))
  (returns (NewWorkNodeStats :type "/Game/Blueprints/WorkNode/FWorkNodeStats Structure"))
  (locals (Stats :type "/Game/Blueprints/WorkNode/FWorkNodeStats Structure") (Map :type "Map of /Game/Blueprints/WorkNode/EWorkNodeConditions Enum to Integer"))
  (bind (_durabilitybreaklimit _durabilitylimit _durabilityresistance _skilllimit _skillresistance _skillbarrechargetime _difficulty _itemdropamount) (break `/Game/Blueprints/WorkNode/FWorkNodeStats` (`local.Stats`)))
  (set `local.Stats` WorkNodeStats)
  (bind _output_get (set `local.Map` WorkNodeConditions))
  (bind _keys (`BlueprintMapLibrary.Map_Keys` _output_get))
  (for _array_element _keys
    (if (!= (`BlueprintMapLibrary.Map_Find` (`local.Map`) _array_element) 0)
      (set `local.Stats` (select `/Game/Blueprints/WorkNode/EWorkNodeConditions` _array_element :`NewEnumerator0` (make `/Game/Blueprints/WorkNode/FWorkNodeStats` _durabilitybreaklimit _durabilitylimit (* _durabilityresistance 0.5) 100.0 5.0 5.0 _difficulty (+ _itemdropamount 1))))))
  (return (`local.Stats`)))

(fn `SkillBarDoneRecharging`
  (`KismetSystemLibrary.K2_ClearAndInvalidateTimerHandle` (`self.SkillBarRechargingTimer`))
  ;[0.1281 0.2865 0.2779] Remove Conditions
  (`BlueprintMapLibrary.Map_Remove` (`self.WorkNodeConditions`) "NewEnumerator0")
  (bind _newworknodestats (`self.ModifyStatsBasedOnConditions` (`self.BaseWorkNodeStats`) (`self.WorkNodeConditions`)))
  (set `self.WorkNodeStats` _newworknodestats)
  (bind _asbp_work_node_ui (cast `/Game/Blueprints/WorkNode/BP_WorkNodeUI` (`WidgetComponent.GetWidget` (`self.UIWidget`))))
  (set `/Game/Blueprints/WorkNode/BP_WorkNodeUI.SkillBreakBarPercent` 1.0 _asbp_work_node_ui))

(fn `UserConstructionScript`)