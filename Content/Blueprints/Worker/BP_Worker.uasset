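; Selectable AI worker character that travels to a work location on a work node and works on it to wear down its durability.
; Tick reroutes if the spot is taken, otherwise snaps the worker in place on arrival and makes it affect navigation.
; A looping timer, scaled by worker stats and node properties, drains a progress bar and reports damage through interface messages.
; Tool swing follows that timer's elapsed fraction through a Timeline.
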(event `self.ReceiveBeginPlay`
  (set `self.MaxMoveSpeed` (`CharacterMovementComponent.MaxWalkSpeed` (`self.CharacterMovement`)))
  (bind _asbp_aiworker_controller (cast `/Game/Blueprints/Worker/BP_AIWorkerController` (`self.GetController`)))
  (set `self.AIController` _asbp_aiworker_controller))

(event `self.ReceiveTick`
  (params (DeltaSeconds :type "Float (single-precision)"))
  (set `self.DeltaSeconds` DeltaSeconds)
  (switch `EPathFollowingStatus` (`AIController.GetMoveStatus` (`self.AIController`))
    (:`Idle`
      (if (`self.IsWorking`)
        ;[0 0.927 1] Tool Animation While Working
        (bind _progresstime (`self.CalculateWorkProgressTime`))
        (bind (_direction _toolrotation) (`Timeline|Timeline` :`NewTime` (/ (`KismetSystemLibrary.K2_GetTimerElapsedTimeHandle` (`self.ProgressTimer`)) _progresstime) :!via `SetNewTime`)
          (:`Update`
            (`SceneComponent.K2_SetRelativeRotation` (`self.Tool`) (`KismetMathLibrary.RotatorFromAxisAndAngle` (0.0 1.0 0.0) (* _toolrotation 360.0)) false false)))))
    (:`Moving`
      (if (`WorkLocationComponent.bIsOccupied` (`self.GoalWorkLocation`))
        ;[1 0 0.007519] What to do if another worker reaches the same location as you before you get there
        (bind (_didfindnewgoal _newgoalworklocation) (`self.RecalculateGoalWorkLocation`))
        (if _didfindnewgoal
          (bind _output_get (set `self.GoalWorkLocation` _newgoalworklocation))
          (`self.MoveToGoalWorkLocation` (`self.GoalLocation`) (`self.GoalWorkNode`) _output_get)
          (else
            (`Controller.StopMovement` (`self.AIController`))
            (set `CharacterMovementComponent.MaxWalkSpeed` 0.0 (`self.CharacterMovement`)) ; For some reason if I don't zero this the workers will still slowly move
          ))
        (else
          ;[1 0 0.007519] What to check while moving towards a goal
          (bind _result (`self.HasReachedGoalLocation`))
          (if _result
            (`self.OnGoalLocationReached`)
            (if (`KismetSystemLibrary.DoesImplementInterface` (`self.GoalWorkNode`) "/Game/Blueprints/WorkNode/BPI_WorkLocationActions.BPI_WorkLocationActions_C")
              (message `/Game/Blueprints/WorkNode/BPI_WorkLocationActions.OnGoalWorkLocationReached` (`self.GoalWorkNode`) (`self.GoalWorkLocation`)))))))))

(event `/Game/Blueprints/Worker/BPI_UnitActions.MoveUnit`
  (params (GoalLocation :type "Vector Structure") (GoalWorkNode :type "/Game/Blueprints/WorkNode/BP_WorkNode Object Reference") (GoalWorkLocation :type "WorkLocationComponent Object Reference"))
  ;[0 0.1466 1] Goal Location Checks
  (`self.MoveToGoalWorkLocation` GoalLocation GoalWorkNode GoalWorkLocation))

(event `OnGoalLocationReached`
  ;[0 0.1466 1] Goal Location Checks
  (`self.OnReachedGoalLocation`))

(event `/Game/Blueprints/WorkNode/BPI_WorkLocationActions.OnGoalWorkLocationLeft`
  ;[0 0.1466 1] Goal Location Checks
  (`self.OnLeftGoalLocation`))

(event `/Game/Blueprints/Worker/BPI_SelectionActions.Select`
  ;[0 0.1466 1] Selection Events
  (`SceneComponent.SetVisibility` (`self.SelectedArrow`) true false))

(event `/Game/Blueprints/Worker/BPI_SelectionActions.Deselect`
  ;[0 0.1466 1] Selection Events
  (`SceneComponent.SetVisibility` (`self.SelectedArrow`) false false))

(event `/Game/Blueprints/WorkNode/BPI_WorkNodeActions.OnDurabilityBreakLimitReached`
  ;[0 0.927 1] Work Node is being destroyed because the durability break limit has been reached
  (`KismetSystemLibrary.K2_ClearAndInvalidateTimerHandle` (`self.ProgressTimer`))
  (set `self.IsWorking` false)
  (bind _asbp_work_progress_bar (cast `/Game/Blueprints/Worker/BP_WorkProgressBar` (`WidgetComponent.GetWidget` (`self.WorkProgressBar`))))
  (`/Game/Blueprints/Worker/BP_WorkProgressBar.SetWorkProgressBarPercent` _asbp_work_progress_bar 1.0)
  (`SceneComponent.K2_SetRelativeRotation` :`self` (`self.Tool`)))

(fn `CalculateWorkProgress`
  (returns (DurabilityDamage :type "Float (double-precision)") (Progress :type "Float (double-precision)"))
  (bind _returnvalue (- (`self.Productivity`) (`/Game/Blueprints/WorkNode/BP_WorkNode.Resistance` (`self.GoalWorkNode`))))
  (return _returnvalue (/ _returnvalue (`/Game/Blueprints/WorkNode/BP_WorkNode.Durability` (`self.GoalWorkNode`)))))

(fn `CalculateWorkProgressTime`
  (returns (ProgressTime :type "Float (double-precision)"))
  (return (* (`self.WorkSpeed`) (`/Game/Blueprints/WorkNode/BP_WorkNode.Difficulty` (`self.GoalWorkNode`)))))

(fn `HasReachedGoalLocation`
  (returns (result :type Boolean))
  (return (<= (`KismetMathLibrary.Vector_Distance` (`self.K2_GetActorLocation`) (`self.GoalLocation`)) (`self.GoalPositionSnapDistance`))))

(fn `MoveToGoalWorkLocation`
  (params (GoalLocation :type "Vector Structure") (GoalWorkNode :type "/Game/Blueprints/WorkNode/BP_WorkNode Object Reference") (GoalWorkLocation :type "WorkLocationComponent Object Reference"))
  (set `self.GoalWorkNode` GoalWorkNode)
  (bind _output_get (set `self.GoalLocation` GoalLocation))
  (set `self.GoalWorkLocation` GoalWorkLocation)
  (set `CharacterMovementComponent.MaxWalkSpeed` (`self.MaxMoveSpeed`) (`self.CharacterMovement`))
  (`AIController.MoveToLocation` (`self.AIController`) _output_get 1.0 false true false true null false)
  (`self.SetCanAffectNavigationGeneration` self false false))

(fn `OnLeftGoalLocation`
  ;[0 0.927 1] Set work variables on Goal Left
  (set `self.IsWorking` false)
  (`SceneComponent.SetVisibility` (`self.WorkProgressBar`) false false)
  (`KismetSystemLibrary.K2_ClearAndInvalidateTimerHandle` (`self.ProgressTimer`)))

(fn `OnReachedGoalLocation`
  ;[1 0 0.007519] Set Navigation Variables on Goal Reached
  (`Controller.StopMovement` (`self.AIController`))
  (set `CharacterMovementComponent.MaxWalkSpeed` 0.0 (`self.CharacterMovement`))
  (`self.K2_SetActorLocationAndRotation` (`self.GoalLocation`) (`KismetMathLibrary.FindLookAtRotation` (`self.GoalLocation`) (`self.K2_GetActorLocation` (`self.GoalWorkNode`)))) ; Snap to Goal Location and Rotation
  (`self.SetCanAffectNavigationGeneration` self true false)
  ;[0 0.927 1] Set Work Variables on Goal Reached
  (set `self.IsWorking` true)
  (`SceneComponent.SetVisibility` (`self.WorkProgressBar`) true false)
  (bind _asbp_work_progress_bar (cast `/Game/Blueprints/Worker/BP_WorkProgressBar` (`WidgetComponent.GetWidget` (`self.WorkProgressBar`))))
  (`/Game/Blueprints/Worker/BP_WorkProgressBar.SetWorkProgressBarPercent` _asbp_work_progress_bar 1.0)
  (bind _progresstime (`self.CalculateWorkProgressTime`))
  (bind _returnvalue (`KismetSystemLibrary.K2_SetTimer` null "UpdateWorkProgress" _progresstime true))
  (set `self.ProgressTimer` _returnvalue))

(fn `OnWorkProgressBarEmpty`
  (`KismetSystemLibrary.K2_ClearAndInvalidateTimerHandle` (`self.WorkProgressBarEmptyTimer`))
  (bind _asbp_work_progress_bar (cast `/Game/Blueprints/Worker/BP_WorkProgressBar` (`WidgetComponent.GetWidget` (`self.WorkProgressBar`))))
  (`/Game/Blueprints/Worker/BP_WorkProgressBar.SetWorkProgressBarPercent` _asbp_work_progress_bar 1.0)
  (if (`KismetSystemLibrary.DoesImplementInterface` (`self.GoalWorkNode`) "/Game/Blueprints/WorkNode/BPI_WorkNodeActions.BPI_WorkNodeActions_C")
    _))

(fn `RecalculateGoalWorkLocation`
  (returns (DidFindNewGoal :type Boolean) (NewGoalWorkLocation :type "WorkLocationComponent Object Reference"))
  (bind (_foundavailable _goalworklocation) (`/Game/Blueprints/WorkNode/BP_WorkNode.FindNearestAvailableWorkLocation` (`self.GoalWorkNode`) (`self.GoalLocation`) (`self.K2_GetActorLocation`)))
  (return _foundavailable _goalworklocation))

(fn `UpdateWorkProgress`
  (locals (BPWorkProgressBar :type "/Game/Blueprints/Worker/BP_WorkProgressBar Object Reference") (DurabilityDamage :type "Float (double-precision)"))
  (`/Engine/EditorBlueprintResources/StandardMacros.IsValid` (`self.GoalWorkNode`)
    (:`Is Valid`
      (bind _asbp_work_progress_bar (cast `/Game/Blueprints/Worker/BP_WorkProgressBar` (`WidgetComponent.GetWidget` (`self.WorkProgressBar`))))
      (set `local.BPWorkProgressBar` _asbp_work_progress_bar)
      (bind (_durabilitydamage _progress) (`self.CalculateWorkProgress`))
      (set `local.DurabilityDamage` _durabilitydamage)
      (bind _returnvalue (- (`/Game/Blueprints/Worker/BP_WorkProgressBar.GetWorkProgressBarPercent` (`local.BPWorkProgressBar`)) _progress))
      (if (`KismetMathLibrary.NearlyEqual_FloatFloat` _returnvalue)
        ;[1 1 1] When Progress Bar Reaches 0
        (`/Game/Blueprints/Worker/BP_WorkProgressBar.SetWorkProgressBarPercent` (`local.BPWorkProgressBar`) 0.0)
        (bind _progresstime (`self.CalculateWorkProgressTime`))
        (bind _returnvalue_2 (`KismetSystemLibrary.K2_SetTimer` null "OnWorkProgressBarEmpty" _progresstime)) ; Set a slight delay before starting work again
        (set `self.WorkProgressBarEmptyTimer` _returnvalue_2)
        (message `/Game/Blueprints/WorkNode/BPI_WorkNodeActions.DecreaseDurabilityBreakLimit` (`self.GoalWorkNode`))
        (else
          ;[1 1 1] Decrease Progress Bar
          (`/Game/Blueprints/Worker/BP_WorkProgressBar.SetWorkProgressBarPercent` (`local.BPWorkProgressBar`) _returnvalue)
          (if (`KismetSystemLibrary.DoesImplementInterface` (`self.GoalWorkNode`) "/Game/Blueprints/WorkNode/BPI_WorkNodeActions.BPI_WorkNodeActions_C")
            (message `/Game/Blueprints/WorkNode/BPI_WorkNodeActions.DurabilityDamageDealtToNode` (`self.GoalWorkNode`) (`local.DurabilityDamage`))))))))

(fn `UserConstructionScript`)