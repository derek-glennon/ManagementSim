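; BP_ResourceItem is a resource pickup that adds to the player's resource count when it reaches the resource shed.
; On BeginPlay, after the parent's logic, it sets HUDLocation to the location of the ManagerController's ResourceShed actor.
; Its OnReachedShed override increments the ResourceMap count for its ResourceType, passes it to UpdateResourceValue on the ManagerController, then calls the parent version.
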(event `self.ReceiveBeginPlay`
  (`parent.ReceiveBeginPlay`)
  (set `self.HUDLocation` (`self.K2_GetActorLocation` (`/Game/Blueprints/Manager/BP_ManagerController.ResourceShed` (`self.ManagerController`)))))

(fn `OnReachedShed`
  (bind _result (`/Engine/EditorBlueprintResources/StandardMacros.IncrementInt` (`BlueprintMapLibrary.Map_Find` (`/Game/Blueprints/Manager/BP_ManagerController.ResourceMap` (`self.ManagerController`)) (`self.ResourceType`)))
    (:`  `
      (`/Game/Blueprints/Manager/BP_ManagerController.UpdateResourceValue` (`self.ManagerController`) (`self.ResourceType`) _result)
      (`parent.OnReachedShed`))))

(fn `UserConstructionScript`
  (`parent.UserConstructionScript`))