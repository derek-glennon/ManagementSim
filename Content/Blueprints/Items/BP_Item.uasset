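; Item pickup actor that lingers briefly after spawning, then flies to a HUD/shed location and destroys itself.
; BeginPlay caches the manager controller and starts a delay timer for MoveToHUD, which disables mesh physics and collision and starts a travel timer.
; Tick scrubs a timeline by that timer's normalized elapsed time to lerp the actor toward HUDLocation, which is not set in these graphs, until OnReachedShed destroys it.
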(event `self.ReceiveBeginPlay`
  (bind _asbp_manager_controller (cast `/Game/Blueprints/Manager/BP_ManagerController` (`GameplayStatics.GetPlayerController` 0)))
  (set `self.ManagerController` _asbp_manager_controller)
  (bind _returnvalue (`KismetSystemLibrary.K2_SetTimer` null "MoveToHUD" (`self.SpawnMoveDelayTime`))) ; Slight delay before moving to HUG
  (set `self.SpawnDelayTimerHandle` _returnvalue))

(event `self.ReceiveTick`
  (params (DeltaSeconds :type "Float (single-precision)"))
  (if (`self.IsTravelingToShed`)
    (bind (_direction _vector_lerp) (`Timeline|MoveToHUD_Timeline` :`NewTime` (/ (`KismetSystemLibrary.K2_GetTimerElapsedTimeHandle` (`self.MoveToShedTimerHandle`)) (`self.MoveToShedTravelTime`)) :!via `SetNewTime`)
      (:`Update`
        (`self.K2_SetActorLocation` (`KismetMathLibrary.VLerp` (`self.ItemStartMoveLocation`) (`self.HUDLocation`) _vector_lerp))))))

(fn `MoveToHUD`
  (`PrimitiveComponent.SetSimulatePhysics` (`self.PickupMesh`) false)
  (`PrimitiveComponent.SetCollisionEnabled` (`self.PickupMesh`) "NoCollision")
  (set `self.ItemStartMoveLocation` (`self.K2_GetActorLocation`))
  (set `self.IsTravelingToShed` true)
  (bind _returnvalue (`KismetSystemLibrary.K2_SetTimer` null "OnReachedShed" (`self.MoveToShedTravelTime`)))
  (set `self.MoveToShedTimerHandle` _returnvalue)
  (return))

(fn `OnReachedShed`
  (set `self.IsTravelingToShed` false)
  (`self.K2_DestroyActor`))

(fn `UserConstructionScript`)