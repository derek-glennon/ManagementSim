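; BP_ItemLootTable picks an item to drop by weighted random selection from the ItemLootTable map of items to weights.
; SetItemToDrop sums the map's weights into ValueSum, then stores the result of ChooseLoot in ItemToDrop.
; ChooseLoot rolls a float up to that sum and walks the keys, subtracting each weight until the roll falls within one.
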(event `SetItemToDrop`
  (bind _totalsum (`self.CalculateSum`))
  (set `self.ValueSum` _totalsum)
  (bind _loot (`self.ChooseLoot`))
  (set `self.ItemToDrop` _loot))

(fn `CalculateSum`
  (returns (TotalSum :type "Float (double-precision)"))
  (locals (RunningTotal :type "Float (double-precision)"))
  (bind _values (`BlueprintMapLibrary.Map_Values` (`self.ItemLootTable`)))
  (for _array_element _values
    (set `local.RunningTotal` (+ _array_element (`local.RunningTotal`))))
  (return (`local.RunningTotal`)))

(fn `ChooseLoot`
  (returns (Loot :type "/Game/Blueprints/Items/BP_Item Class Reference"))
  (locals (RandomValue :type "Float (double-precision)" :default 0.0))
  (set `local.RandomValue` (`KismetMathLibrary.RandomFloatInRange` 0.0 (`self.ValueSum`)))
  (bind _keys (`BlueprintMapLibrary.Map_Keys` (`self.ItemLootTable`)))
  (for _array_element _keys
    (bind _value (`BlueprintMapLibrary.Map_Find` (`self.ItemLootTable`) _array_element))
    (if (<= (`local.RandomValue`) _value)
      (return _array_element)
      (else
        (set `local.RandomValue` (- (`local.RandomValue`) _value))))))